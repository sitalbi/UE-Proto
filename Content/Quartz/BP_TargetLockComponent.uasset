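; Target lock component that shows a screen-space marker widget on the current lock target.
; On BeginPlay it adds an unattached screen-space WidgetComponent to its owner.
; Locking creates a WB_TargetLock widget and places it once at the target location, raised by half the draw height, with no per-tick update here.
; Unlocking clears the widget.
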(event `self.ReceiveBeginPlay`
  (bind _returnvalue (`|AddComponentByClass` :`self` (`self.GetOwner`) :`Class` "/Script/UMG.WidgetComponent" :`bManualAttachment` true))
  (`WidgetComponent.SetWidgetSpace` _returnvalue "Screen")
  (`WidgetComponent.SetDrawSize` _returnvalue (50.0 50.0))
  (set `self.TargetLockWidgetComponent` _returnvalue))

(event `self.OnLockTarget`
  (`self.RenderTargetLockWidget` true))

(event `self.OnUnlockTarget`
  (`self.RenderTargetLockWidget` false))

(fn `RenderTargetLockWidget`
  (params (RenderWidget :type Boolean))
  (bind _targetlockwidgetcomponent (`self.TargetLockWidgetComponent`))
  (if RenderWidget
    (bind _returnvalue (`|CreateWidget` "/Game/Quartz/UI/WB_TargetLock.WB_TargetLock_C"))
    (`WidgetComponent.SetWidget` _targetlockwidgetcomponent _returnvalue)
    (`SceneComponent.K2_SetWorldLocation` _targetlockwidgetcomponent (+ (`self.GetTargetLocation`) (`KismetMathLibrary.MakeVector` 0.0 0.0 (/ (`.Y` (`KismetMathLibrary.BreakVector2D` (`WidgetComponent.GetDrawSize` (`self.TargetLockWidgetComponent`)))) 2.0))) false false)
    (else
      (`WidgetComponent.SetWidget` (`self.TargetLockWidgetComponent`) null))))