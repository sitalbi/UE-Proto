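; Interaction component that shows a screen-space interaction prompt at the world location of the current interactable.
; BeginPlay adds a manually attached widget component to the owner to host the prompt.
; Interactable added and removed events refresh it, creating a new WB_PlayerInteraction each time it shows and clearing it when none remain.
; The first entry in OverlappingInteractables sets the position, which updates only on those events.
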(event `self.ReceiveBeginPlay`
  (bind _returnvalue (`|AddComponentByClass` :`self` (`self.GetOwner`) :`Class` "/Script/UMG.WidgetComponent" :`bManualAttachment` true))
  (`WidgetComponent.SetWidgetSpace` _returnvalue "Screen")
  (`WidgetComponent.SetDrawSize` _returnvalue (128.0 200.0))
  (set `self.InteractionWidgetComponent` _returnvalue))

(event `self.OnInteractableAdded`
  (params (NewInteractable :type "QuartzInteractableInterface Interface (by ref)"))
  (`self.RenderInteractionWidget` true))

(event `self.OnInteractableRemoved`
  (params (RemovedInteractable :type "QuartzInteractableInterface Interface (by ref)"))
  (`self.RenderInteractionWidget` (`KismetArrayLibrary.Array_IsNotEmpty` (`self.OverlappingInteractables`))))

(fn `GetCurrentInteractablePosition`
  (returns (InteractablePosition :type "Vector Structure"))
  (if (`KismetArrayLibrary.Array_IsNotEmpty` (`self.OverlappingInteractables`))
    (bind _asactor (cast `Actor` (`|GetArrayItem` (`self.OverlappingInteractables`))))
    (return (`Actor.K2_GetActorLocation` _asactor))
    (else
      (return (0.0 0.0 0.0)))))

(fn `RenderInteractionWidget`
  (params (showWidget :type Boolean :default true))
  (bind _interactionwidgetcomponent (`self.InteractionWidgetComponent`))
  (if showWidget
    (bind _returnvalue (`|CreateWidget` "/Game/Quartz/UI/WB_PlayerInteraction.WB_PlayerInteraction_C"))
    (`WidgetComponent.SetWidget` _interactionwidgetcomponent _returnvalue)
    (`SceneComponent.K2_SetWorldLocation` _interactionwidgetcomponent (`self.GetCurrentInteractablePosition`) false false)
    (else
      (`WidgetComponent.SetWidget` (`self.InteractionWidgetComponent`) null))))