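; Anim notify state that detects melee weapon hits for the Quartz player character during an attack animation window.
; Each tick sphere-traces between the weapon mesh's base and top sockets, ignoring actors already hit since the window began.
; Each new hit actor is recorded and sent as the target of an Event.Attack.Hit gameplay event to the owner, leaving the hit response to that event's listeners.
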(fn `Received_NotifyBegin`
  (params (MeshComp :type "SkeletalMeshComponent Object Reference") (Animation :type "AnimSequenceBase Object Reference") (TotalDuration :type "Float (single-precision)") (EventReference :type "AnimNotifyEventReference Structure (by ref)"))
  (returns (ReturnValue :type Boolean))
  (`KismetArrayLibrary.Array_Clear` (`self.HitActors`))
  (return false))

(fn `Received_NotifyEnd`
  (params (MeshComp :type "SkeletalMeshComponent Object Reference") (Animation :type "AnimSequenceBase Object Reference") (EventReference :type "AnimNotifyEventReference Structure (by ref)"))
  (returns (ReturnValue :type Boolean))
  (return false))

(fn `Received_NotifyTick`
  (params (MeshComp :type "SkeletalMeshComponent Object Reference") (Animation :type "AnimSequenceBase Object Reference") (FrameDeltaTime :type "Float (single-precision)") (EventReference :type "AnimNotifyEventReference Structure (by ref)"))
  (returns (ReturnValue :type Boolean))
  (locals (HitActor :type "Actor Object Reference") (OwnerActor :type "Actor Object Reference"))
  (bind _output_get (set `local.OwnerActor` (`ActorComponent.GetOwner` MeshComp)))
  (bind _asquartz_player_character (cast `QuartzPlayerCharacter` _output_get))
  (bind _weaponmeshcomp (`QuartzPlayerCharacter.WeaponMeshComp` _asquartz_player_character))
  (bind _outhits (`KismetSystemLibrary.SphereTraceMulti` _asquartz_player_character (`SceneComponent.GetSocketLocation` _weaponmeshcomp (`self.WeaponBaseSocket`)) (`SceneComponent.GetSocketLocation` _weaponmeshcomp (`self.WeaponTopSocket`)) 15.0 (`self.Trace Channel`) false (`self.HitActors`) "None" true (struct :`R` 1.0 :`A` 1.0) (struct :`G` 1.0 :`A` 1.0) 2.0))
  (for _array_element _outhits
    (bind (_bblockinghit _binitialoverlap _time _distance _location _impactpoint _normal _impactnormal _physmat _hitactor) (`GameplayStatics.BreakHitResult` _array_element))
    (bind _output_get_2 (set `local.HitActor` _hitactor))
    (if (not (`KismetArrayLibrary.Array_Contains` (`self.HitActors`) _hitactor))
      (`KismetArrayLibrary.Array_Add` (`self.HitActors`) _output_get_2)
      (`AbilitySystemBlueprintLibrary.SendGameplayEventToActor` (`local.OwnerActor`) (struct :`TagName` "Event.Attack.Hit") (make `GameplayEventData` (struct :`TagName` "Event.Attack.Hit") (`local.OwnerActor`) (`local.HitActor`)))))
  (return false))