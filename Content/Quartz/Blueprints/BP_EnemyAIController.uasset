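; AI controller for enemies in Quartz that tracks the player through perception.
; On begin play it binds to AIPerception target updates and reacts only to the Quartz player character.
; A successful sense stores the player as current target, flags it visible and records its location.
; A lost sense clears the visible flag and keeps the stimulus location as last known, leaving the target set.
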(event `self.ReceiveBeginPlay`
  (add `AIPerceptionComponent.OnTargetPerceptionUpdated` (`self.AIPerception`) (delegate `OnTargetPerceptionUpdated`)))

(event `OnTargetPerceptionUpdated`
  (params (Actor :type "Actor Object Reference") (Stimulus :type "AIStimulus Structure"))
  (bind (_age _expirationage _strength _stimuluslocation _receiverlocation _tag _bsuccessfullysensed) (break `AIStimulus` Stimulus))
  (`/Engine/EditorBlueprintResources/StandardMacros.IsValid` Actor
    (:`Is Valid`
      (bind _asquartz_player_character (cast `QuartzPlayerCharacter` Actor))
      (if _bsuccessfullysensed
        (bind _output_get (set `self.CurrentTarget` _asquartz_player_character))
        (set `self.bCanSeeTarget` true)
        (set `self.LastKnownLcoation` (`self.K2_GetActorLocation` _output_get))
        (else
          (set `self.bCanSeeTarget` false)
          (set `self.LastKnownLcoation` _stimuluslocation))))))

(fn `UserConstructionScript`)