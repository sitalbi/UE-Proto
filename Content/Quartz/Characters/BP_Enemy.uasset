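; Base enemy character that can be locked onto, flashes when hit and ragdolls on death.
; BeginPlay swaps mesh materials for dynamic instances, whose FlashAmount a timeline drives on each hit cue.
; OnDeath stops movement, disables capsule collision, simulates mesh physics, hides the health bar, then destroys the actor after a delay.
; Lock-on functions supply fixed distances and a spine socket location, refusing targeting once QuartzHealthComponent reports death.
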(event `self.ReceiveBeginPlay`
  (`KismetArrayLibrary.Array_Clear` (`self.MaterialInstances`))
  (for (_array_element _array_index) (`MeshComponent.GetMaterials` (`self.Mesh`))
    (bind _returnvalue (`KismetMaterialLibrary.CreateDynamicMaterialInstance` _array_element))
    (`KismetArrayLibrary.Array_Add` (`self.MaterialInstances`) _returnvalue)
    (`PrimitiveComponent.SetMaterial` (`self.Mesh`) _array_index _returnvalue)))

(event `StartHitFlash`
  (bind (_direction _flash) (`Timeline|TL_HitFlash` :!via `PlayFromStart`)
    (:`Update`
      (for _array_element (`self.MaterialInstances`)
        (`MaterialInstanceDynamic.SetScalarParameterValue` _array_element "FlashAmount" _flash)))))

(event `self.OnHitCue`
  (`self.StartHitFlash`) ; TODO: Add particles when hit too
)

(event `self.OnDeath`
  (bind _mesh (`self.Mesh`))
  (`CharacterMovementComponent.DisableMovement` (`self.CharacterMovement`))
  (`PrimitiveComponent.SetCollisionEnabled` (`self.CapsuleComponent`) "NoCollision")
  (`PrimitiveComponent.SetCollisionProfileName` _mesh "Ragdoll" false)
  (`PrimitiveComponent.SetCollisionResponseToAllChannels` (`self.Capsule`) "ECR_Ignore")
  (`PrimitiveComponent.SetCollisionResponseToChannel` (`self.Mesh`) "ECC_Pawn" "ECR_Ignore")
  (`PrimitiveComponent.SetSimulatePhysics` _mesh true)
  (`KismetSystemLibrary.Delay` 0.2)
  (`QuartzHealthComponent.HideHealthBar` (`self.QuartzHealthComponent`))
  (`KismetSystemLibrary.Delay` 5.0)
  (`self.K2_DestroyActor`))

(fn `CanBeLockedOn`
  (returns (ReturnValue :type Boolean))
  (return (not (`QuartzHealthComponent.IsDead` (`self.QuartzHealthComponent`)))))

(fn `GetLockOnDistance`
  (returns (ReturnValue :type "Float (single-precision)"))
  (return 1500.0))

(fn `GetLockOnLocation`
  (returns (ReturnValue :type "Vector Structure"))
  (return (`SceneComponent.GetSocketLocation` (`self.Mesh`) "spine_05")))

(fn `GetLockOutDistance`
  (returns (ReturnValue :type "Float (single-precision)"))
  (return 2000.0))

(fn `UserConstructionScript`)